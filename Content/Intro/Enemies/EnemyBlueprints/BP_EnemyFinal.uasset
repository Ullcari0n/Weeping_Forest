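; Weeping-angel style horror enemy that chases the player with AI MoveTo, freezing only when looked at with the flashlight on and unobstructed.
; Tick tests view direction by dot product and occlusion by line trace; being newly looked at swaps its static-mesh pose.
; When unseen and distant, it periodically relocates to random navmesh points around the player.
; Prolonged staring triggers flashlight flicker if battery allows, while getting too close ends the game.
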(event Custom|Change%20Pose
  (bind _posemeshes (Variables|Default|GetPoseMeshes))
  (if (not (Variables|Default|GetIsGameOver))
    ;[0.15 0.15 0.15 0.5] Increment current pose index by 1, and reset to 0 if reach length of poses array
    (bind _result (Math|Integer|IncrementInt (Variables|Default|GetCurrentPoseIndex))
      (:%20%20
        (bind _output_get (Variables|Default|SetCurrentPoseIndex (Math|Integer|%(Integer) _result (Utilities|Array|Length _posemeshes))))
        ;[0.15 0.15 0.15 0.5] Set mesh of enemy to new pose
        (Components|StaticMesh|SetStaticMesh (Variables|Default|GetEnemy%20Pose) (Utilities|Array|Get(acopy) _posemeshes _output_get))))))

(event Custom|Move%20Enemy%20Randomly
  (Variables|Default|SetMoveTimer 0.0)
  (Transformation|SetActorLocation (.ProjectedLocation (AI|Navigation|ProjectPointtoNavigation (+ (* (Math|Vector|Normalize (Math|Vector|MakeVector (Math|Random|RandomFloatinRange -1.0 1.0) (Math|Random|RandomFloatinRange -1.0 1.0) 0.0)) (Math|Random|RandomFloatinRange 1.5e+03 3e+03)) (Transformation|GetActorLocation (Game|GetPlayerCharacter 0))) 0 0 "0, 0, 0")) false false))

(event EventBeginPlay
  ;[0.15 0.15 0.15 0.5] Spawn enemy at random location, get player reference, and set enemy speed
  (CallFunction|MoveEnemyRandomly)
  (bind _asbp_first_person_character (Utilities|Casting|CastToBP_FirstPersonCharacter (Game|GetPlayerCharacter 0)))
  (Variables|Default|SetPlayerRef _asbp_first_person_character)
  (Variables|/Script/Engine.FloatingPawnMovement|SetMaxSpeed (Variables|Default|GetFloatingPawnMovement) (Variables|Default|GetEnemySpeed)))

(event Collision|EventActorBeginOverlap
  (params (OtherActor :type Actor%20Object%20Reference)))

(event EventTick
  (params (DeltaSeconds :type Float%20%28single-precision%29))
  (bind _self self)
  (bind _self_2 self)
  (bind _playerref (Variables|Default|GetPlayerRef))
  (bind _playerref_2 (Variables|Default|GetPlayerRef))
  (bind _playerref_3 (Variables|Default|GetPlayerRef))
  (bind _playerref_4 (Variables|Default|GetPlayerRef))
  (bind _returnvalue (Transformation|GetActorLocation _playerref))
  (bind (_x _y) (Math|Vector|BreakVector _returnvalue))
  (if (not (Variables|Default|GetIsGameOver))
    (bind _output_get (Variables|Default|SetMoveTimer (+ DeltaSeconds (Variables|Default|GetMoveTimer))))
    (if (>= _output_get 5.0)
      (if (>= (Transformation|GetDistanceTo (Variables|Default|GetPlayerRef)) 1.5e+03)
        (if (Variables|Default|GetIsSeen)
          _
          (else
            (CallFunction|MoveEnemyRandomly)))))
    ;[0.15 0.15 0.15 0.5] Enemy always rotated towards player
    (Transformation|SetActorRotation (Math|Rotator|FindLookatRotation (Transformation|GetActorLocation) (Transformation|GetActorLocation (Variables|Default|GetPlayerRef))))
    ;[0.15 0.15 0.15 0.5] Prevent enemy from rotating on any other axis than vertical (Z) axis
    (Transformation|SetActorRotation (Math|Rotator|MakeRotator 0.0 0.0 (.Yaw (Math|Rotator|BreakRotator (Transformation|GetActorRotation)))))
    ;[0.15 0.15 0.15 0.5] Is player looking in direction of enemy
    (bind _asplayer_controller (Utilities|Casting|CastToPlayerController (Pawn|GetController _playerref_2)))
    (if (>= (Math|Vector|DotProduct (Math|Vector|GetUnitDirection(Vector) (Transformation|GetActorLocation) (Transformation|GetActorLocation _playerref_2)) (Math|Vector|GetForwardVector (Pawn|GetControlRotation _asplayer_controller :!class /Script/Engine.Controller))) -0.8)
      (Variables|Default|SetIsInLineOfSight false)
      (Development|PrintString "not being looked at by player: enemy can move" false false)
      ;[0.15 0.15 0.15 0.5] Enemy moves towards player
      (AI|AIMoveTo self (Math|Vector|MakeVector _x _y 0.0) 0 5.0 false :!label _label
        (:then
          (Variables|Default|SetIsSeen false)
          (Variables|Default|SetFlickerTriggered false)
          (Variables|Default|SetSeenTimer 0.0)))
      (else
        ;[0.15 0.15 0.15 0.5] If player wasn't looking at enemy but then looks at enemy, change enemy pose
        (if (Variables|Default|GetIsInLineOfSight)
          _
          (else
            (CallFunction|ChangePose)))
        (Variables|Default|SetIsInLineOfSight true)
        (if (Variables|/Game/FirstPerson/Blueprints/BP_FirstPersonCharacter.BP_FirstPersonCharacter_C|GetIsFlashlightOn _playerref_4)
          ;[0.15 0.15 0.15 0.5] Is there an object between player and enemy
          (bind _returnvalue_2 (Collision|LineTraceByChannel (Transformation|GetActorLocation) (Transformation|GetActorLocation _playerref_4) "TraceTypeQuery1" false 0 "None"))
          (if _returnvalue_2
            (Development|PrintString "object between player and enemy: enemy can move" false false)
            (goto _label)
            (else
              (Development|PrintString "enemy cannot move" false false)
              ;[0.15 0.15 0.15 0.5] Enemy does not move
              (AI|AIMoveTo _self "0, 0, 0" _self 5.0 false
                (:then
                  (Variables|Default|SetIsSeen true)))))
          (else
            (Development|PrintString "flashlight is off: enemy can move" false false)
            (goto _label)))))
    (if (<= (Transformation|GetDistanceTo (Variables|Default|GetPlayerRef)) 1.5e+02)
      ;[0.15 0.15 0.15 0.5] Game Over: Stops player movement, disables input, and turns on flashlight (to see monster)
      (Development|PrintString "Game Over")
      (AI|AIMoveTo _self_2 "0, 0, 0" _self_2 5.0 false
        (:then
          (Variables|Default|SetIsGameOver true)
          (Input|DisableInput (Game|GetPlayerCharacter 0) (Game|GetPlayerController (Variables|/Script/Engine.Pawn|GetPlayerState (Variables|Default|GetPlayerRef))))
          (Variables|/Game/FirstPerson/Blueprints/BP_FirstPersonCharacter.BP_FirstPersonCharacter_C|SetIsFlickering _playerref_3 false)
          (Rendering|SetVisibility (Variables|/Game/FirstPerson/Blueprints/BP_FirstPersonCharacter.BP_FirstPersonCharacter_C|GetSpotLight _playerref_3) true true)
          (Variables|/Script/Engine.SkeletalMeshComponent|SetGlobalAnimRateScale (Variables|/Script/Engine.Character|GetMesh (Variables|Default|GetPlayerRef)) 0.0)))
      (else
        ;[0.15 0.15 0.15 0.5] If player looks at enemy for more than 3s, and flashlight battery is more than 15%, flashlight flickers
        (bind _output_get_2 (Variables|Default|SetSeenTimer (+ (Variables|Default|GetSeenTimer) DeltaSeconds)))
        (if (>= _output_get_2 3.0)
          (if (not (< (Variables|/Game/FirstPerson/Blueprints/BP_FirstPersonCharacter.BP_FirstPersonCharacter_C|GetBatteryLevel (Variables|Default|GetPlayerRef)) 15.0))
            (if (not (Variables|Default|GetFlickerTriggered))
              (Variables|Default|SetFlickerTriggered true)
              (Default|StartFlashlightFlicker (Variables|Default|GetPlayerRef)))))))))

(fn ConstructionScript)