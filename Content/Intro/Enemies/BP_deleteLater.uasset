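; Scratch enemy Blueprint, named for deletion, that holds an unfinished test for whether the player is looking at this actor.
; BeginPlay caches the first-person character, while Tick and overlap events do nothing.
; Disconnected logic compares the direction to the player against the control rotation by dot product, then uses a Visibility trace to print when the player faces it unobstructed.
; Nothing calls that check or its debug print of the dot value.
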(event EventBeginPlay
  (bind _asbp_first_person_character (Utilities|Casting|CastToBP_FirstPersonCharacter (Game|GetPlayerCharacter 0)))
  (Variables|Default|SetPlayerRef _asbp_first_person_character))

(event Collision|EventActorBeginOverlap
  (params (OtherActor :type Actor%20Object%20Reference)))

(event EventTick
  (params (DeltaSeconds :type Float%20%28single-precision%29)))

(fn ConstructionScript)