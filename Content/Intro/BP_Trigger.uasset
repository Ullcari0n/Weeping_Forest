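; BP_Trigger is an intro-level trigger that takes a battery from the first-person player and switches a point light, which starts dark.
; On player overlap, the first battery fills the socket, and every later overlap raises the count without checking for a battery.
; Below three, it clears the player's battery flag and prints a warning.
; From three on, a FlipFlop toggles the light between saved intensity and zero.
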(event EventBeginPlay
  (bind _pointlight (Variables|Default|GetPointLight))
  (Variables|Default|SetLightIntensity (Variables|/Script/Engine.LightComponentBase|GetIntensity _pointlight))
  (Rendering|Components|Light|SetIntensity _pointlight 0.0)
  ;[0.15 0.15 0.15 0.5] Save Player Instance
  (bind _asbp_first_person_character (Utilities|Casting|CastToBP_FirstPersonCharacter (Game|GetPlayerCharacter 0))
    (:then
      (Variables|Default|SetPlayer _asbp_first_person_character))
    (:CastFailed
      (Development|PrintString "Not using the correct character"))))

(event Collision|EventActorBeginOverlap
  (params (OtherActor :type Actor%20Object%20Reference))
  (if (Actor|ActorHasTag OtherActor "Player")
    (if (Variables|Default|GetHasBatteryInSocket)
      (Variables|Default|SetBatteryCount (+ (Variables|Default|GetBatteryCount) 1))
      (if (<= 3 (Variables|Default|GetBatteryCount)) :!label _label
        ;[0.15 0.15 0.15 0.5] Player interraction with light
        (bind _isa (Utilities|FlowControl|FlipFlop)
          (:A
            _)
          (:B
            _))
        (Rendering|Components|Light|SetIntensity (Variables|Default|GetPointLight) (Math|Float|SelectFloat (Variables|Default|GetLightIntensity) 0.0 _isa))
        (else
          (Development|PrintString "Player hasnt put enough batteries in the car")
          (Variables|/Game/FirstPerson/Blueprints/BP_FirstPersonCharacter.BP_FirstPersonCharacter_C|SetHasBattery (Variables|Default|GetPlayer) false)))
      (elif (Variables|/Game/FirstPerson/Blueprints/BP_FirstPersonCharacter.BP_FirstPersonCharacter_C|GetHasBattery (Variables|Default|GetPlayer))
        (Variables|/Game/FirstPerson/Blueprints/BP_FirstPersonCharacter.BP_FirstPersonCharacter_C|SetHasBattery (Variables|Default|GetPlayer) false)
        (Variables|Default|SetHasBatteryInSocket true)
        (Variables|Default|SetBatteryCount (+ (Variables|Default|GetBatteryCount) 1))
        (goto _label)
        (else
          (Development|PrintString "Player has No Battery"))))))

(event EventTick
  (params (DeltaSeconds :type Float%20%28single-precision%29)))

(fn ConstructionScript)